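; BP_Environment is the scenery actor that dresses the level with the environment stored in the AberrationGameInstance.
; On BeginPlay it reads that Environment data and sets the Background sprite and the Ground material.
; It gives the player and enemy platforms the same platform material.
; Nothing updates after startup, and nothing is applied if the game instance cast fails.
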(event EventBeginPlay
  (bind _asaberration_game_instance (Utilities|Casting|CastToAberrationGameInstance (Game|GetGameInstance)))
  (Utilities|FlowControl|Sequence
    (:then_0
      (Rendering|Components|Sprite|SetSprite (Variables|Default|GetBackground) (.background (Variables|/Game/ProjectAberration/Gameplay/AberrationGameInstance.AberrationGameInstance_C|GetEnvironment _asaberration_game_instance))))
    (:then_1
      (Rendering|Material|SetMaterial (Variables|Default|GetGround) 0 (.groundmaterial (Variables|/Game/ProjectAberration/Gameplay/AberrationGameInstance.AberrationGameInstance_C|GetEnvironment _asaberration_game_instance))))
    (:then_2
      (Rendering|Material|SetMaterial (Variables|Default|GetPlatform_Player) 0 (.platformsmaterial (Variables|/Game/ProjectAberration/Gameplay/AberrationGameInstance.AberrationGameInstance_C|GetEnvironment _asaberration_game_instance)))
      (Rendering|Material|SetMaterial (Variables|Default|GetPlatform_Enemy) 0 (.platformsmaterial (Variables|/Game/ProjectAberration/Gameplay/AberrationGameInstance.AberrationGameInstance_C|GetEnvironment _asaberration_game_instance))))))

(event Collision|EventActorBeginOverlap
  (params (OtherActor :type Actor%20Object%20Reference)))

(event EventTick
  (params (DeltaSeconds :type Float%20%28single-precision%29)))

(fn ConstructionScript)