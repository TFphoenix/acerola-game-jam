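; BP_Aberration is a creature assembled from its equipped parts, which supply both its look and its combat stats.
; On BeginPlay it layers Paper2D sprites in back, body and front passes with increasing translucent sort priority, adding components for back and front and setting the existing body sprite.
; It then sums part stats, including keyed attack and defense multipliers, into StatsComponent and sets current health to the total.
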(event EventBeginPlay
  (CallFunction|InitializeBodyParts)
  (CallFunction|InitializeStats))

(event Collision|EventActorBeginOverlap
  (params (OtherActor :type Actor%20Object%20Reference)))

(event EventTick
  (params (DeltaSeconds :type Float%20%28single-precision%29)))

(fn ConstructionScript)

(fn InitializeBodyParts
  (bind _body_sprite (Variables|Default|GetBody_Sprite))
  (bind _currentsortpriority (LocalVariables|GetCurrentSortPriority))
  (bind _currentsortpriority_2 (LocalVariables|GetCurrentSortPriority))
  (bind _currentsortpriority_3 (LocalVariables|GetCurrentSortPriority))
  (Utilities|FlowControl|Sequence
    (:then_0
      ;[1 1 1] Back Parts
      (for _array_element (Variables|Default|GetEquipedParts)
        (Utilities|IsValid (.backsprite (Variables|/Script/ProjectAberration.BodyPartDataAsset|GetSprites _array_element))
          (:Is%20Valid
            (bind _returnvalue (AddComponent|AddPaperSpriteComponent false))
            (Rendering|Components|Sprite|SetSprite _returnvalue (.backsprite (Variables|/Script/ProjectAberration.BodyPartDataAsset|GetSprites _array_element)))
            (Rendering|SetTranslucentSortPriority _returnvalue _currentsortpriority_2)
            (Math|Integer|IncrementInt _currentsortpriority_2)))))
    (:then_1
      ;[1 1 1] Body Part
      (for _array_element_2 (Variables|Default|GetEquipedParts)
        (Utilities|IsValid (.bodysprite (Variables|/Script/ProjectAberration.BodyPartDataAsset|GetSprites _array_element_2))
          (:Is%20Valid
            (Rendering|Components|Sprite|SetSprite _body_sprite (.bodysprite (Variables|/Script/ProjectAberration.BodyPartDataAsset|GetSprites _array_element_2)))
            (Rendering|SetTranslucentSortPriority _body_sprite _currentsortpriority_3)
            (Math|Integer|IncrementInt _currentsortpriority_3)))))
    (:then_2
      ;[1 1 1] Front Parts
      (for _array_element_3 (Variables|Default|GetEquipedParts)
        (Utilities|IsValid (.frontsprite (Variables|/Script/ProjectAberration.BodyPartDataAsset|GetSprites _array_element_3))
          (:Is%20Valid
            (bind _returnvalue_2 (AddComponent|AddPaperSpriteComponent false))
            (Rendering|Components|Sprite|SetSprite _returnvalue_2 (.frontsprite (Variables|/Script/ProjectAberration.BodyPartDataAsset|GetSprites _array_element_3)))
            (Rendering|SetTranslucentSortPriority _returnvalue_2 _currentsortpriority)
            (Math|Integer|IncrementInt _currentsortpriority)))))))

(fn InitializeStats
  (bind _statscomponent (Variables|Default|GetStatsComponent))
  (for _array_element (Variables|Default|GetEquipedParts)
    (Utilities|FlowControl|Sequence
      (:then_0
        (LocalVariables|SetHealth_Sum (+ (LocalVariables|GetHealth_Sum) (.health (Variables|/Script/ProjectAberration.BodyPartDataAsset|GetStats _array_element)))))
      (:then_1
        (LocalVariables|SetAttack_Sum (+ (LocalVariables|GetAttack_Sum) (.attack (Variables|/Script/ProjectAberration.BodyPartDataAsset|GetStats _array_element)))))
      (:then_2
        (LocalVariables|SetCriticalChance_Sum (+ (LocalVariables|GetCriticalChance_Sum) (.criticalchance (Variables|/Script/ProjectAberration.BodyPartDataAsset|GetStats _array_element)))))
      (:then_3
        (LocalVariables|SetEvasionChance_Sum (+ (LocalVariables|GetEvasionChance_Sum) (.evasionchance (Variables|/Script/ProjectAberration.BodyPartDataAsset|GetStats _array_element)))))
      (:then_4
        (bind _keys (Utilities|Map|Keys (.attackmultipliers (Variables|/Script/ProjectAberration.BodyPartDataAsset|GetStats _array_element))))
        (for _array_element_2 _keys
          (Utilities|Map|Add (LocalVariables|GetAttackMultipliers_Sum) _array_element_2 (+ (.Value (Utilities|Map|Find (.attackmultipliers (Variables|/Script/ProjectAberration.BodyPartDataAsset|GetStats _array_element)) _array_element_2)) (.Value (Utilities|Map|Find (LocalVariables|GetAttackMultipliers_Sum) _array_element_2))))))
      (:then_5
        (bind _keys_2 (Utilities|Map|Keys (.defensemultipliers (Variables|/Script/ProjectAberration.BodyPartDataAsset|GetStats _array_element))))
        (for _array_element_3 _keys_2
          (Utilities|Map|Add (LocalVariables|GetDefenseMultipliers_Sum) _array_element_3 (+ (.Value (Utilities|Map|Find (.defensemultipliers (Variables|/Script/ProjectAberration.BodyPartDataAsset|GetStats _array_element)) _array_element_3)) (.Value (Utilities|Map|Find (LocalVariables|GetDefenseMultipliers_Sum) _array_element_3))))))))
  (Utilities|Struct|SetmembersinPartStats (Variables|/Script/ProjectAberration.StatsComponent|GetGeneralStats _statscomponent) (LocalVariables|GetHealth_Sum) (LocalVariables|GetAttack_Sum) (LocalVariables|GetCriticalChance_Sum) (LocalVariables|GetEvasionChance_Sum) (LocalVariables|GetAttackMultipliers_Sum) (LocalVariables|GetDefenseMultipliers_Sum))
  (Variables|/Script/ProjectAberration.StatsComponent|SetCurrentHealth _statscomponent (LocalVariables|GetHealth_Sum)))