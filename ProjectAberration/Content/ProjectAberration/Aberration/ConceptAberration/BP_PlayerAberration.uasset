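; BP_PlayerAberration is the player's aberration Blueprint, which takes its equipped body parts from saved player state in the game instance.
; On BeginPlay it copies Player.CurrentBodyParts from AberrationGameInstance into EquipedParts, then calls the parent BeginPlay.
; If the game instance cast fails, the parent BeginPlay is never called.
; The construction script only defers to the parent, and the overlap and tick events are disabled.
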(event EventBeginPlay
  (bind _asaberration_game_instance (Utilities|Casting|CastToAberrationGameInstance (Game|GetGameInstance)))
  (Variables|Default|SetEquipedParts (.currentbodyparts (Variables|/Game/ProjectAberration/Gameplay/AberrationGameInstance.AberrationGameInstance_C|GetPlayer _asaberration_game_instance)))
  (|CallParentFunction))

(event Collision|EventActorBeginOverlap
  (params (OtherActor :type Actor%20Object%20Reference))
  (|CallParentFunction OtherActor) ; This node is disabled and will not be called.\nDrag off pins to build functionality.
)

(event EventTick
  (params (DeltaSeconds :type Float%20%28single-precision%29))
  (|CallParentFunction DeltaSeconds) ; This node is disabled and will not be called.\nDrag off pins to build functionality.
)

(fn ConstructionScript
  (|CallParentFunction))